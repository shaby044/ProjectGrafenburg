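; Player character that handles Enhanced Input movement, look, jump, flashlight toggle, crouch, lean and sprint, and adds a stamina widget to the viewport on BeginPlay.
; Timelines blend capsule height for crouching and capsule roll for leaning, reversing on release.
; Sprint press and release run retriggerable-delay loops that drain or regenerate stamina, switching walk speed and ending the sprint when stamina runs out.
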(event `self.ReceiveBeginPlay`
  ;[1 1 1] Cast UI to Screen
  (bind _returnvalue (`|CreateWidget` "/Game/UI/WP_Stamina.WP_Stamina_C" (`GameplayStatics.GetPlayerController` 0)))
  (`UserWidget.AddToViewport` _returnvalue 0)
  ;[1 1 1] Use Enhanced Input
  (bind _asplayer_controller (cast `PlayerController` (`self.GetController`)))
  (bind _returnvalue_2 (pcsubsystem `EnhancedInputLocalPlayerSubsystem` _asplayer_controller))
  (`/Engine/EditorBlueprintResources/StandardMacros.IsValid` _returnvalue_2
    (:`Is Valid`
      (`EnhancedInputSubsystemInterface.AddMappingContext` _returnvalue_2 "/Game/Blueprints/Player/Inputs/IMC_InGame.IMC_InGame" 0 (struct)))))

(event `EnhancedInput|/Game/Blueprints/Player/Inputs/IA_Look`
  (params (ActionValue :type "Vector2D Structure") (ElapsedSeconds :type "Float (double-precision)") (TriggeredSeconds :type "Float (double-precision)") (InputAction :type "InputAction Object Reference" :default "/Game/Blueprints/Player/Inputs/IA_Look.IA_Look"))
  ;[1 1 1] Look (Camera Input) (Mouse Axis)
  (:`Triggered`
    (`self.AddControllerYawInput` ActionValue_X)
    (`self.AddControllerPitchInput` ActionValue_Y)))

(event `EnhancedInput|/Game/Blueprints/Player/Inputs/IA_Move`
  (params (ActionValue :type "Vector2D Structure") (ElapsedSeconds :type "Float (double-precision)") (TriggeredSeconds :type "Float (double-precision)") (InputAction :type "InputAction Object Reference" :default "/Game/Blueprints/Player/Inputs/IA_Move.IA_Move"))
  (bind (_returnvalue_roll _returnvalue_pitch _returnvalue_yaw) (`KismetMathLibrary.BreakRotator` (`self.GetControlRotation`)))
  (bind (_returnvalue_roll_2 _returnvalue_pitch_2 _returnvalue_yaw_2) (`KismetMathLibrary.BreakRotator` (`self.GetControlRotation`)))
  ;[1 1 1] Movement (W, A, S, D)
  (:`Triggered`
    (`self.AddMovementInput` (`KismetMathLibrary.GetRightVector` (`KismetMathLibrary.MakeRotator` _returnvalue_roll_2 0.0 _returnvalue_yaw_2)) ActionValue_X)
    (`self.AddMovementInput` (`KismetMathLibrary.GetForwardVector` (`KismetMathLibrary.MakeRotator` 0.0 0.0 _returnvalue_yaw)) ActionValue_Y)))

(event `EnhancedInput|/Game/Blueprints/Player/Inputs/IA_Jump`
  (params (ActionValue :type Boolean) (ElapsedSeconds :type "Float (double-precision)") (TriggeredSeconds :type "Float (double-precision)") (InputAction :type "InputAction Object Reference" :default "/Game/Blueprints/Player/Inputs/IA_Jump.IA_Jump"))
  ;[1 1 1] Jump (Spacebar)
  (:`Triggered`
    (`self.Jump`))
  (:`Completed`
    (`self.StopJumping`)))

(event `EnhancedInput|/Game/Blueprints/Player/Inputs/IA_ToggleFlashlight`
  (params (ActionValue :type Boolean) (ElapsedSeconds :type "Float (double-precision)") (TriggeredSeconds :type "Float (double-precision)") (InputAction :type "InputAction Object Reference" :default "/Game/Blueprints/Player/Inputs/IA_ToggleFlashlight.IA_ToggleFlashlight"))
  ;[1 1 1] Toggle Flashlight
  (:`Completed`
    (`SceneComponent.ToggleVisibility` (`self.SpotLight`) false)))

(event `EnhancedInput|/Game/Blueprints/Player/Inputs/IA_Crouch`
  (params (ActionValue :type Boolean) (ElapsedSeconds :type "Float (double-precision)") (TriggeredSeconds :type "Float (double-precision)") (InputAction :type "InputAction Object Reference" :default "/Game/Blueprints/Player/Inputs/IA_Crouch.IA_Crouch"))
  (bind _charactermovement (`self.CharacterMovement`))
  ;[1 1 1] Crouch (C)
  (:`Triggered`
    (set `CharacterMovementComponent.MaxWalkSpeed` 150.0 _charactermovement)
    (bind (_direction _lean_track) (`Timeline|Timeline_1` :!label _label)
      (:`Update`
        (`CapsuleComponent.SetCapsuleHalfHeight` (`self.CapsuleComponent`) (`KismetMathLibrary.Lerp` (`self.StandingHalfHeight`) (`self.CrouchHalfHeight`) _lean_track) true))))
  (:`Completed`
    (set `CharacterMovementComponent.MaxWalkSpeed` 450.0 _charactermovement)
    (goto _label :!via `Reverse`)))

(event `EnhancedInput|/Game/Blueprints/Player/Inputs/IA_LeanLeft`
  (params (ActionValue :type Boolean) (ElapsedSeconds :type "Float (double-precision)") (TriggeredSeconds :type "Float (double-precision)") (InputAction :type "InputAction Object Reference" :default "/Game/Blueprints/Player/Inputs/IA_LeanLeft.IA_LeanLeft"))
  (:`Triggered`
    (bind (_direction _lean_track) (`Timeline|Timeline_0` :!label _label_2)
      (:`Update`
        (`SceneComponent.K2_SetRelativeRotation` (`self.CapsuleComponent`) (`KismetMathLibrary.MakeRotator` (`KismetMathLibrary.Lerp` 0.0 45.0 _lean_track)) false false))))
  (:`Completed`
    (goto _label_2 :!via `Reverse`)))

(event `Drain Stamina`
  (bind _stamina (`self.stamina`))
  (set `self.stamina` (- _stamina 2))
  (if (< _stamina 0)
    (set `self.isSprinting` false)
    (set `CharacterMovementComponent.MaxWalkSpeed` 450.0 (`self.CharacterMovement`))
    (else
      (`KismetSystemLibrary.PrintString` (`KismetStringLibrary.Conv_IntToString` _stamina)))))

(event `EnhancedInput|/Game/Blueprints/Player/Inputs/IA_LeanRight`
  (params (ActionValue :type Boolean) (ElapsedSeconds :type "Float (double-precision)") (TriggeredSeconds :type "Float (double-precision)") (InputAction :type "InputAction Object Reference" :default "/Game/Blueprints/Player/Inputs/IA_LeanRight.IA_LeanRight"))
  (:`Triggered`
    (bind (_direction _lean_track) (`Timeline|Timeline` :!label _label_3)
      (:`Update`
        (`SceneComponent.K2_SetRelativeRotation` (`self.CapsuleComponent`) (`KismetMathLibrary.MakeRotator` (`KismetMathLibrary.Lerp` 0.0 -45.0 _lean_track)) false false))))
  (:`Completed`
    (goto _label_3 :!via `Reverse`)))

(event `EnhancedInput|/Game/Blueprints/Player/Inputs/IA_Sprint`
  (params (ActionValue :type Boolean) (ElapsedSeconds :type "Float (double-precision)") (TriggeredSeconds :type "Float (double-precision)") (InputAction :type "InputAction Object Reference" :default "/Game/Blueprints/Player/Inputs/IA_Sprint.IA_Sprint"))
  (bind _issprinting (`self.isSprinting`))
  (bind _charactermovement (`self.CharacterMovement`))
  (:`Started`
    (set `self.isSprinting` true)
    (set `CharacterMovementComponent.MaxWalkSpeed` 700.0 _charactermovement :!label _label_4)
    (`KismetSystemLibrary.RetriggerableDelay` 0.2)
    (`self.Drain Stamina`)
    (if _issprinting
      (goto _label_4)))
  (:`Completed`
    (set `self.isSprinting` false)
    (set `CharacterMovementComponent.MaxWalkSpeed` 450.0 _charactermovement :!label _label_5)
    (`KismetSystemLibrary.RetriggerableDelay` 0.2)
    (`self.Raise Stamina`)
    (if (not _issprinting)
      (goto _label_5))))

(event `Raise Stamina`
  (bind _stamina (`self.stamina`))
  (if (not (`self.FullStamina`))
    (set `self.stamina` (+ (`self.stamina`) 1))
    (`KismetSystemLibrary.PrintString` (`KismetStringLibrary.Conv_IntToString` _stamina))
    (if (>= _stamina 100)
      (set `self.FullStamina` true))))

(fn `UserConstructionScript`)